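; Player character Blueprint that routes input to telekinesis, weapon system and tripwire trap components, plus jumping and dashing.
; BeginPlay adds the player HUD widget and starts a looping timer for AutoDOF, which line-traces from the camera to set depth-of-field focal distance.
; Dash launches the character along scaled horizontal velocity; an alternative timeline-lerped teleport dash is present but unconnected.
; A WalkRunSFX function plays footstep audio, varying pitch by speed.
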(event `self.ReceiveBeginPlay`
  (`|ExecutionSequence`
    (:`then_0`
      (bind _returnvalue (`|CreateWidget` "/Game/MainGame/Player/UI/WBP_Player.WBP_Player_C"))
      (`UserWidget.AddToViewport` _returnvalue 0))
    (:`then_1`
      (`KismetSystemLibrary.K2_SetTimer` null "AutoDOF" 0.2 true))))

(event `InputAction|Telekenesis`
  (params (Key :type "Key Structure"))
  ;[1 1 1] Ability: Telekinesis
  (:`Pressed`
    (`TelekinesisComponent.StartTelekinesis` (`self.TelekinesisComponent`))
    (`GameplayStatics.SpawnSoundAtLocation` "/Game/MainGame/Player/Assets/Audio/Telekinesis/pull.pull" (`self.K2_GetActorLocation`) (struct) 1.0 1.0 0.0 null null))
  (:`Released`
    (`TelekinesisComponent.ReleaseTelekineticObject` (`self.TelekinesisComponent`))
    (`GameplayStatics.SpawnSoundAtLocation` "/Game/MainGame/Player/Assets/Audio/Telekinesis/push.push" (`self.K2_GetActorLocation`) (struct) 1.0 1.0 0.0 null null)))

(event `InputAction|Shoot`
  (params (Key :type "Key Structure"))
  (bind _weaponsystemcomponent (`self.WeaponSystemComponent`))
  (:`Pressed`
    (`WeaponSystemComponent.Shoot` _weaponsystemcomponent))
  (:`Released`
    (`WeaponSystemComponent.StopShoot` _weaponsystemcomponent)))

(event `InputAction|Reload`
  (params (Key :type "Key Structure"))
  (:`Pressed`
    (`WeaponSystemComponent.Reload` (`self.WeaponSystemComponent`))))

(event `InputAction|Jump`
  (params (Key :type "Key Structure"))
  ;[1 1 1] Weapon System
  (:`Pressed`
    (`self.Jump`)
    (set `self.isJumping` true))
  (:`Released`
    (`self.StopJumping`)
    (set `self.isJumping` false)))

(event `InputAction|Dash`
  (params (Key :type "Key Structure"))
  (bind (_returnvalue_x _returnvalue_y) (`KismetMathLibrary.BreakVector` (`self.GetVelocity`)))
  ;[1 1 1] Weapon System
  (:`Pressed`
    (`self.LaunchCharacter` (* (`KismetMathLibrary.MakeVector` _returnvalue_x _returnvalue_y) 10))))

(event `InputAction|SwitchGun`
  (params (Key :type "Key Structure"))
  ;[1 1 1] Weapon System
  (:`Pressed`
    (`WeaponSystemComponent.switchGun` (`self.WeaponSystemComponent`))))

(event `Dash Begin`
  (bind (_returnvalue_x _returnvalue_y) (`KismetMathLibrary.BreakVector` (`self.GetActorForwardVector`)))
  (bind (_returnvalue_x_2 _returnvalue_y_2) (`KismetMathLibrary.BreakVector` (`self.K2_GetActorLocation`)))
  ;[1 1 1] Weapon System
  (`self.MoveOverTime` (+ (`KismetMathLibrary.MakeVector` _returnvalue_x_2 _returnvalue_y_2) (* (`KismetMathLibrary.MakeVector` _returnvalue_x _returnvalue_y) 1200.0))))

(event `MoveOverTime`
  (params (Location :type "Vector Structure"))
  (bind (_returnvalue_x _returnvalue_y) (`KismetMathLibrary.BreakVector` (`self.K2_GetActorLocation`)))
  ;[1 1 1] Weapon System
  (bind _output_get (set `self.Current Location` (`KismetMathLibrary.MakeVector` _returnvalue_x _returnvalue_y)))
  (bind _returnvalue_roll (`KismetMathLibrary.BreakRotator` (`KismetMathLibrary.FindLookAtRotation` _output_get Location)))
  (`self.K2_SetActorRotation` (`KismetMathLibrary.MakeRotator` _returnvalue_roll))
  (bind (_direction _location_alpha) (`Timeline|Dash Timeline` :!via `PlayFromStart`)
    (:`Update`
      (bind (_returnvalue_x_2 _returnvalue_y_2) (`KismetMathLibrary.BreakVector` (`KismetMathLibrary.VLerp` (`self.Current Location`) Location _location_alpha)))
      (`self.K2_SetActorLocation` (`KismetMathLibrary.MakeVector` _returnvalue_x_2 _returnvalue_y_2) false true))))

(event `InputAction|SetTrap`
  (params (Key :type "Key Structure"))
  ;[1 1 1] Weapon System
  (:`Pressed`
    (`TripWireComponent.SetupTrap` (`self.TripWire`))))

(event `AutoDOF`
  (bind _playerviewcamera (`self.PlayerViewCamera`))
  (bind _returnvalue (`SceneComponent.K2_GetComponentLocation` _playerviewcamera))
  ;[1 1 1] AutoDOF
  (bind (_outhit _returnvalue_2) (`KismetSystemLibrary.LineTraceSingle` _returnvalue (+ _returnvalue (* (`SceneComponent.GetForwardVector` _playerviewcamera) 10000.0)) "TraceTypeQuery1"))
  (if _returnvalue_2
    (set `self.FocusLocation` (`KismetMathLibrary.VSize` (- (`.Location` (`GameplayStatics.BreakHitResult` _outhit)) (`SceneComponent.K2_GetComponentLocation` (`self.PlayerViewCamera`)))))
    (set `CameraComponent.PostProcessSettings` (make `PostProcessSettings` :`DepthOfFieldFstop` 1.0 :`DepthOfFieldMinFstop` 11.0 :`DepthOfFieldFocalDistance` (`self.FocusLocation`)) (`self.PlayerViewCamera`))))

(fn `UserConstructionScript`)

(fn `WalkRunSFX`
  (params (walkrunspeed :type "Float (double-precision)"))
  (if (> walkrunspeed 750.0)
    (bind _returnvalue (`GameplayStatics.CreateSound2D` "/Game/MainGame/Player/Assets/Audio/ExoSuit/SC_walk.SC_walk" 1.0 walkrunspeed 0.0 null))
    (`AudioComponent.Play` _returnvalue 0.0)
    (else
      (bind _returnvalue_2 (`GameplayStatics.CreateSound2D` "/Game/MainGame/Player/Assets/Audio/ExoSuit/SC_walk.SC_walk" 1.0 1.0 0.0 null))
      (`AudioComponent.Play` _returnvalue_2 0.0))))