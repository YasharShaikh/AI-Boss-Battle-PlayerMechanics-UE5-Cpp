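; BP_LargeTO is a large telekinetic object that breaks apart when it hits something while in a specific state.
; Its mesh hit event checks that state and an IsHit flag, then plays an impact sound and spawns a concrete destruction effect at its location.
; It returns to its pool immediately rather than being destroyed, while IsHit is set only after a delay matching the sound's length.
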(event `self.MeshComponent.OnComponentHit`
  (params (HitComponent :type "PrimitiveComponent Object Reference") (OtherActor :type "Actor Object Reference") (OtherComp :type "PrimitiveComponent Object Reference") (NormalImpulse :type "Vector Structure") (Hit :type "HitResult Structure (by ref)"))
  (bind _returnvalue (`self.K2_GetActorLocation`))
  (bind _sound (`self.Sound`))
  (if (== (`self.GetCurrentState`) 3)
    (if (not (`self.isHit`))
      (`|ExecutionSequence`
        (:`then_0`
          (bind _returnvalue_2 (message `AnimationDataModel.GetPlayLength` _sound))
          (`GameplayStatics.PlaySoundAtLocation` _sound _returnvalue (struct) 1.0 1.0 0.0 null null null null)
          (`KismetSystemLibrary.Delay` _returnvalue_2)
          (set `self.isHit` true))
        (:`then_1`
          (`GameplayStatics.SpawnEmitterAtLocation` "/Game/AssetPack/Realistic_Starter_VFX_Pack_Vol2/Particles/Destruction/P_Destruction_Concrete.P_Destruction_Concrete" _returnvalue (struct) (1.0 1.0 1.0) true "AutoRelease")
          (`self.ReturnToPool`))))))

(fn `UserConstructionScript`)